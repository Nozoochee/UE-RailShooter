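; PC_RSPlayerCon is a player controller that lets a gamepad aim by moving the mouse cursor.
; Any key press updates IsUsingGamepad according to whether that key is a gamepad key.
; While that flag is set, the AimRight and AimUp axis events both drive one shared SetMouseLocation call.
; It offsets the cursor by axis value, AimSpeed and frame delta time, clamped to the viewport.
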(event `InputAction|AnyKey` :consume false :paused true
  (params (Key :type "Key Structure"))
  ;[0.3968 0.3968 0.3968] Every time we press something, see if it's gamepad
  (:`Pressed`
    (set `self.isUsingGamepad` (`KismetInputLibrary.Key_IsGamepadKey` Key))))

(event `InputAxis|AimRight`
  (params (AxisValue :type "Float (single-precision)"))
  (bind (_locationx _locationy) (`self.GetMousePosition`))
  (bind (_sizex _sizey) (`self.GetViewportSize`))
  ;[0.3968 0.3968 0.3968] Controller aim
  (if (`self.isUsingGamepad`)
    (`self.SetMouseLocation` (`KismetMathLibrary.Clamp` (`KismetMathLibrary.FTrunc` (+ (* AxisValue (`self.AimSpeed`) (`GameplayStatics.GetWorldDeltaSeconds`)) _locationx)) 0 _sizex) (`KismetMathLibrary.Clamp` (`KismetMathLibrary.FTrunc` (+ _locationy (* (`self.AimSpeed`) (stale `InputAxis|AimUp` AxisValue) (`GameplayStatics.GetWorldDeltaSeconds`)))) 0 _sizey) :!label _label)))

(event `InputAxis|AimUp`
  (params (AxisValue :type "Float (single-precision)"))
  ;[0.3968 0.3968 0.3968] Controller aim
  (if (`self.isUsingGamepad`)
    (goto _label)))

(fn `UserConstructionScript`)