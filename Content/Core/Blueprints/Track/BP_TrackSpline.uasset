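; BP_TrackSpline is a spline track that moves a reference point along itself at forward speed while active.
; Each tick it advances distance, broadcasts when a spline point is reached, and either loops or deactivates at the end.
; Branch entries at reached points can deactivate it, position the next track at a chosen start point and call SwitchTrack on the player pawn.
; The construction script labels the track and numbers each spline point with text.
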(event `self.ReceiveTick`
  (params (DeltaSeconds :type "Float (single-precision)"))
  ;[0.3968 0.3968 0.3968] Calculate how far we move based on Speed
  (if (`self.isActive`)
    (set `self.Distance` (+ (* DeltaSeconds (`self.ForwardSpeed`)) (`self.Distance`)))
    (`self.MoveRefPoint`)
    (`self.CheckReachedNextPoint`)
    (`self.HandleLooping`)))

(fn `CheckBranch`
  (locals (NewTrack :type "/Game/Core/Blueprints/Track/BP_TrackSpline Object Reference"))
  (bind _newtrack (`local.NewTrack`))
  (bind _newtrack_2 (`local.NewTrack`))
  (for _array_element (`self.Branches`)
    (bind (_nexttrack _branchpoint _shouldbranch _startpoint) (break `/Game/Core/Blueprints/Track/S_Branch` _array_element))
    ;[0.3968 0.3968 0.3968] Should we branch
    (if (and (== (`self.LastReachedSplinePoint`) _branchpoint) _shouldbranch)
      (set `self.isActive` false)
      ;[0.3968 0.3968 0.3968] Initialize new track
      (set `local.NewTrack` _nexttrack)
      (bind (_returnvalue_location _returnvalue_rotation) (`KismetMathLibrary.BreakTransform` (`SplineComponent.GetTransformAtSplinePoint` (`/Game/Core/Blueprints/Track/BP_TrackSpline.Spline` _newtrack) _startpoint "World" false)))
      (`SceneComponent.K2_SetWorldLocationAndRotation` (`/Game/Core/Blueprints/Track/BP_TrackSpline.ReferencePoint` _newtrack) _returnvalue_location _returnvalue_rotation false false)
      ;;[1 1 1] Making it work even if we re-join a track at a later point
      (set `/Game/Core/Blueprints/Track/BP_TrackSpline.LastReachedSplinePoint` _startpoint _newtrack_2)
      (set `/Game/Core/Blueprints/Track/BP_TrackSpline.Distance` (`SplineComponent.GetDistanceAlongSplineAtSplinePoint` (`/Game/Core/Blueprints/Track/BP_TrackSpline.Spline` _newtrack_2) _startpoint) (`local.NewTrack`))
      ;[0.3968 0.3968 0.3968] Let Player know we switched
      (bind _asbp_base_player (cast `/Game/Core/Blueprints/Player/BP_BasePlayer` (`GameplayStatics.GetPlayerPawn` 0)))
      (`/Game/Core/Blueprints/Player/BP_BasePlayer.SwitchTrack` _asbp_base_player (`local.NewTrack`))
      (return))))

(fn `CheckReachedNextPoint`
  ;[0.3968 0.3968 0.3968] Are we ahead of the next spline point?
  ;[0.3968 0.3968 0.3968] Increase counter, call dispatcher to let everyone know we reached a new point, check if we branch here
  (if (>= (`self.Distance`) (`SplineComponent.GetDistanceAlongSplineAtSplinePoint` (`self.Spline`) (+ (`self.LastReachedSplinePoint`) 1)))
    (bind _result (`/Engine/EditorBlueprintResources/StandardMacros.IncrementInt` (`self.LastReachedSplinePoint`))
      (:`  `
        (`self.OnSplinePointReached` _result)
        (`self.CheckBranch`)))))

(fn `HandleLooping`
  ;[1 1 1] If you want to loop, make sure the first and last spline point are at the same position
  ;;[1 1 1] Have we reached the end of the spline?
  (if (>= (`self.Distance`) (`SplineComponent.GetSplineLength` (`self.Spline`)))
    (if (`self.isLooping`)
      (set `self.Distance` 0.0)
      (else
        (set `self.isActive` false)))))

(fn `MoveRefPoint`
  (bind _spline (`self.Spline`))
  (bind _distance (`self.Distance`))
  ;[0.3968 0.3968 0.3968] Move ReferencePoint to our newly calculated Distance
  (`SceneComponent.K2_SetWorldLocationAndRotation` (`self.ReferencePoint`) (`SplineComponent.GetLocationAtDistanceAlongSpline` _spline _distance "World") (`SplineComponent.GetRotationAtDistanceAlongSpline` _spline _distance "World") false false))

(fn `UserConstructionScript`
  (bind _spline (`self.Spline`))
  (`TextRenderComponent.K2_SetText` (`self.Track_Name`) (`self.TrackName`))
  ;[0.3968 0.3968 0.3968] Draws the text above each spline point (click on Add Text Render Component to change settings)
  (for _index (range (`SplineComponent.GetNumberOfSplinePoints` _spline))
    (bind _returnvalue (`AddComponent|NODE_AddTextRenderComponent-0` :`RelativeTransform` (`KismetMathLibrary.MakeTransform` (`KismetMathLibrary.MakeVector` (.x (`SplineComponent.GetLocationAtSplinePoint` _spline _index "Local")) (.y (`SplineComponent.GetLocationAtSplinePoint` _spline _index "Local")) (+ (.z (`SplineComponent.GetLocationAtSplinePoint` _spline _index "Local")) 100.0)) (struct :`Yaw` -180.0))))
    (`TextRenderComponent.K2_SetText` _returnvalue (`KismetTextLibrary.Conv_IntToText` _index))))