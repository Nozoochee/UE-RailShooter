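; Blueprint function library with screen-space helpers for testing whether a world location is within a player's view.
; IsInView projects the location to screen coordinates, checks both axes against the viewport size, and returns the result with the screen position.
; IsFloatInBounds supplies the below-minimum and above-maximum flags for each axis.
; The test is bounds-only, with no occlusion check and no use of the projection's success flag.
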(fn `isFloatInBounds`
  (params (In :type "Float (double-precision)") (Min :type "Float (double-precision)") (Max :type "Float (double-precision)"))
  (returns (BelowMin :type Boolean) (AboveMax :type Boolean))
  (return (< In Min) (> In Max)))

(fn `IsInView`
  (params (PlayerController :type "PlayerController Object Reference") (Loc :type "Vector Structure"))
  (returns (ReturnValue :type Boolean) (ScreenPos :type "Vector2D Structure"))
  (locals (sp :type "Vector2D Structure"))
  (bind (_x _y) (`KismetMathLibrary.BreakVector2D` (`local.sp`)))
  (bind (_returnvalue_x _returnvalue_y) (`KismetMathLibrary.BreakVector2D` (`WidgetLayoutLibrary.GetViewportSize` (`local.PlayerController`))))
  (bind (_belowmin _abovemax) (`self.isFloatInBounds` _y 0.0 _returnvalue_y (`local.PlayerController`)))
  (bind (_belowmin_2 _abovemax_2) (`self.isFloatInBounds` _x 0.0 _returnvalue_x (`local.PlayerController`)))
  (set `local.sp` (`GameplayStatics.ProjectWorldToScreen` PlayerController Loc))
  (return (not (or _belowmin_2 _abovemax_2 _belowmin _abovemax)) (`local.sp`)))