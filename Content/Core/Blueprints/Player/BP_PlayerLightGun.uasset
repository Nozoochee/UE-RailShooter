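; Player pawn for a light-gun shooter on a track, built on BP_BasePlayer logic and firing at whatever sits under the cursor.
; Shooting applies hitscan damage via a cursor trace and plays a timeline that drives recoil pitch.
; While movement is allowed, Tick moves the player, eases camera FOV with track speed, and aims the gun mesh at the cursor hit point with recoil added on top.
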(event `self.ReceiveBeginPlay`
  ;[0.3968 0.3968 0.3968] See BP_BasePlayer
  (`parent.ReceiveBeginPlay`))

(event `InputAction|Shoot`
  (params (Key :type "Key Structure"))
  ;[0.3968 0.3968 0.3968] Shoot (RecoilRotPitch is used in RotateGunToCrosshair function)
  (:`Pressed`
    (`self.StartShooting`)
    (bind (_direction _y) (`Timeline|GunRecoil` :!via `PlayFromStart`)
      (:`Update`
        (set `self.RecoilRotPitch` _y)))))

(event `self.ReceiveTick`
  (params (DeltaSeconds :type "Float (single-precision)"))
  ;[0.3968 0.3968 0.3968] Tick
  (if (`self.CanMove`)
    (`self.MoveActor` (`self.ShouldRotateWithTrack`))
    (`self.AdjustCamera`)
    (`self.RotateGunToCrosshair`)))

(fn `AdjustCamera`
  ;[0.3968 0.3968 0.3968] Changes FOV slightly depending on speed
  (set `CameraComponent.FieldOfView` (`KismetMathLibrary.FInterpTo` (`CameraComponent.FieldOfView` (`self.Camera`)) (`KismetMathLibrary.MapRangeClamped` (`/Game/Core/Blueprints/Track/BP_TrackSpline.ForwardSpeed` (`self.Track`)) 0.0 500.0 90.0 100.0) (`GameplayStatics.GetWorldDeltaSeconds`) 4.0) (`self.Camera`)))

(fn `RotateGunToCrosshair`
  (locals (NormalizedMousePos :type "Vector2D Structure"))
  (bind (_hitresult _returnvalue) (`PlayerController.GetHitResultUnderCursorByChannel` (`GameplayStatics.GetPlayerController` 0) "TraceTypeQuery3" false))
  ;[0.3968 0.3968 0.3968] Uses the ShootPoint to get a hit result, then rotate gun towards it. Lastly add the recoil on top
  (if _returnvalue
    (`SceneComponent.K2_SetWorldRotation` (`self.GunMesh`) (`KismetMathLibrary.MakeRotator` (.roll (`KismetMathLibrary.FindLookAtRotation` (`SceneComponent.K2_GetComponentLocation` (`self.GunMesh`)) (`.Location` (`GameplayStatics.BreakHitResult` _hitresult)))) (+ (.pitch (`KismetMathLibrary.FindLookAtRotation` (`SceneComponent.K2_GetComponentLocation` (`self.GunMesh`)) (`.Location` (`GameplayStatics.BreakHitResult` _hitresult)))) (`self.RecoilRotPitch`)) (.yaw (`KismetMathLibrary.FindLookAtRotation` (`SceneComponent.K2_GetComponentLocation` (`self.GunMesh`)) (`.Location` (`GameplayStatics.BreakHitResult` _hitresult))))) false false)))

(fn `StartShooting`
  (bind (_hitresult _returnvalue) (`PlayerController.GetHitResultUnderCursorByChannel` (`GameplayStatics.GetPlayerController` 0) "TraceTypeQuery1" true))
  ;[0.3968 0.3968 0.3968] Trace under the cursor and if we hit something deal damage to it
  (if _returnvalue
    (`GameplayStatics.ApplyDamage` (`.HitActor` (`GameplayStatics.BreakHitResult` _hitresult)) 5.0 null self)))

(fn `UserConstructionScript`)