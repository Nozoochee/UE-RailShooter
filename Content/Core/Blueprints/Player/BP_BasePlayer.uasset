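; Base player actor that follows a track, activating it on play and switching to new tracks at branches.
; MoveActor interpolates location, and optionally rotation, toward the active Track's reference point at separate speeds.
; Damage, including contact with simple enemies, goes to the health component, triggering camera shake and brief invincibility.
; The health component's death dispatcher deactivates the track, destroys the player and opens the main menu.
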(event `self.ReceiveBeginPlay`
  ;[0.3968 0.3968 0.3968] Begin Play
  (set `/Game/Core/Blueprints/Track/BP_TrackSpline.isActive` true (`self.Track`))
  ;;[1 1 1] HealthComp does the damage calculation, so it knows when we died and then calls a dispatcher, which then makes us call the "Die" event
  (add `/Game/Core/Blueprints/AC_HealthComp.OnDeath` (`self.AC_HealthComp`) (delegate `Die`)))

(event `Die`
  ;[0.3968 0.3968 0.3968] Begin Play
  ;;[1 1 1] HealthComp does the damage calculation, so it knows when we died and then calls a dispatcher, which then makes us call the "Die" event
  (set `/Game/Core/Blueprints/Track/BP_TrackSpline.isActive` false (`self.Track`))
  (`self.K2_DestroyActor`)
  ;[1 0.0102 0.03009] Go back to main menu when dead
  (`GameplayStatics.OpenLevel` "/Game/MainMenu/MainMenu"))

(event `self.ReceiveAnyDamage`
  (params (Damage :type "Float (single-precision)") (DamageType :type "DamageType Object Reference") (InstigatedBy :type "Controller Object Reference") (DamageCauser :type "Actor Object Reference"))
  ;[0.3968 0.3968 0.3968] Take damage
  (if (not (`self.isInvincible`))
    ;;[1 1 1] HealthComp decreases our health
    (`/Game/Core/Blueprints/AC_HealthComp.TakeDamage` (`self.AC_HealthComp`) Damage DamageType InstigatedBy DamageCauser)
    ;;[1 1 1] Camera shake
    (`GameplayStatics.PlayWorldCameraShake` "/Game/Core/Blueprints/Player/CS_PlayerHit.CS_PlayerHit_C" (`self.K2_GetActorLocation`) 0.0 1000.0)
    ;;[1 1 1] Make us invincible for 1 sec
    (set `self.isInvincible` true)
    (`KismetSystemLibrary.Delay` 1.0)
    (set `self.isInvincible` false)))

(event `self.Hitbox.OnComponentBeginOverlap`
  (params (OverlappedComponent :type "PrimitiveComponent Object Reference") (OtherActor :type "Actor Object Reference") (OtherComp :type "PrimitiveComponent Object Reference") (OtherBodyIndex :type Integer) (bFromSweep :type Boolean) (SweepResult :type "HitResult Structure (by ref)"))
  ;[0.3968 0.3968 0.3968] Contact with enemy
  (cast `/Game/Core/Blueprints/Enemies/BP_SimpleEnemy` OtherActor)
  (`GameplayStatics.ApplyDamage` self 5.0))

(event `SwitchTrack`
  (params (NewTrack :type "/Game/Core/Blueprints/Track/BP_TrackSpline Object Reference"))
  ;[0.3968 0.3968 0.3968] Switching Track (called in BP_Track when branching)
  (bind _output_get (set `self.Track` NewTrack))
  (set `/Game/Core/Blueprints/Track/BP_TrackSpline.isActive` true _output_get))

(fn `MoveActor`
  (params (RotateWithTrack :type Boolean))
  ;[0.3968 0.3968 0.3968] This moves the entire actor to the Track's reference point. You can adjust location and rotation speed seperately
  (`self.K2_SetActorLocation` (`KismetMathLibrary.VInterpTo` (`self.K2_GetActorLocation`) (`SceneComponent.K2_GetComponentLocation` (`/Game/Core/Blueprints/Track/BP_TrackSpline.ReferencePoint` (`self.Track`))) (`GameplayStatics.GetWorldDeltaSeconds`) 6.0))
  (if (`local.RotateWithTrack`)
    (`self.K2_SetActorRotation` (`KismetMathLibrary.RInterpTo` (`self.K2_GetActorRotation`) (`SceneComponent.K2_GetComponentRotation` (`/Game/Core/Blueprints/Track/BP_TrackSpline.ReferencePoint` (`self.Track`))) (`GameplayStatics.GetWorldDeltaSeconds`) 3.0))))

(fn `UserConstructionScript`)