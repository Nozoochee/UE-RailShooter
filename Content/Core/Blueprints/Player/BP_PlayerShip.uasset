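; Player ship for a rail shooter, derived from BP_BasePlayer, that moves along a track and fires BP_Projectile from its Muzzle socket toward a cursor-traced aim point.
; Camera-relative input offsets the Hitbox, clamped inside screen margins via world-to-screen projection, with automatic return when off-screen.
; Each tick while CanMove also adjusts spring arm length from track speed and capsule-traces static geometry to apply collision damage unless invincible.
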(event `InputAxis|MoveRight`
  (params (AxisValue :type "Float (single-precision)"))
  ;[0.3968 0.3968 0.3968] Inputs (Movement is based on camera rotation, so moving right will always move you right on screen)
  (set `self.MoveRightDelta` (* (`self.GetActorRightVector` (`GameplayStatics.GetPlayerCameraManager` 0)) (* AxisValue (`self.Speed`)))))

(event `StartShooting`
  (bind _returnvalue (`SceneComponent.GetSocketLocation` (`self.StaticMesh`) "Muzzle"))
  ;[0.3968 0.3968 0.3968] Shoot (Make sure your mesh has a Socket called "Muzzle")
  (`|SpawnActorFromClass` "/Game/Core/Blueprints/BP_Projectile.BP_Projectile_C" (`KismetMathLibrary.MakeTransform` _returnvalue (`KismetMathLibrary.FindLookAtRotation` _returnvalue (`SceneComponent.K2_GetComponentLocation` (`self.AimPoint`)))) "AlwaysSpawn" "OverrideRootScale" self null))

(event `InputAxis|MoveUp`
  (params (AxisValue :type "Float (single-precision)"))
  ;[0.3968 0.3968 0.3968] Inputs (Movement is based on camera rotation, so moving right will always move you right on screen)
  (set `self.MoveUpDelta` (* (`self.GetActorUpVector` (`GameplayStatics.GetPlayerCameraManager` 0)) (* AxisValue (`self.Speed`)))))

(event `InputAction|Shoot`
  (params (Key :type "Key Structure"))
  ;[0.3968 0.3968 0.3968] Inputs (Movement is based on camera rotation, so moving right will always move you right on screen)
  (:`Pressed`
    (`self.StartShooting`)))

(event `self.ReceiveBeginPlay`
  ;[0.3968 0.3968 0.3968] Begin Play (see BP_BasePlayer)
  (`parent.ReceiveBeginPlay`))

(event `self.ReceiveTick`
  (params (DeltaSeconds :type "Float (single-precision)"))
  ;[0.3968 0.3968 0.3968] Tick
  (if (`self.CanMove`)
    (`self.MoveActor` (`self.ShouldRotateWithTrack`))
    (`self.MoveShip`)
    (`self.SetAimPointLoc`)
    (`self.AdjustCamera`)
    (`self.TraceAround`)))

(fn `AdjustCamera`
  ;[0.3968 0.3968 0.3968] Adjusts camera distance based on forward speed
  (set `SpringArmComponent.TargetArmLength` (`KismetMathLibrary.FInterpTo` (`SpringArmComponent.TargetArmLength` (`self.SpringArm`)) (`KismetMathLibrary.MapRangeClamped` (`/Game/Core/Blueprints/Track/BP_TrackSpline.ForwardSpeed` (`self.Track`)) 0.0 500.0 50.0 300.0) (`GameplayStatics.GetWorldDeltaSeconds`) 4.0) (`self.SpringArm`)))

(fn `ClampToScreen`
  (params (DeltaRight :type "Vector Structure") (DeltaUp :type "Vector Structure"))
  (returns (ClampedDelta :type "Vector Structure"))
  (locals (ScreenPos :type "Vector2D Structure") (Sidemargin :type "Float (double-precision)") (Topmargin :type "Float (double-precision)"))
  (bind _deltaright (`local.DeltaRight`))
  (bind _deltaup (`local.DeltaUp`))
  (bind (_x _y) (`KismetMathLibrary.BreakVector2D` (`WidgetLayoutLibrary.GetViewportSize`)))
  (bind (_x_2 _y_2) (`KismetMathLibrary.BreakVector2D` (`local.ScreenPos`)))
  (bind (_x_3 _y_3) (`KismetMathLibrary.BreakVector2D` (`WidgetLayoutLibrary.GetViewportSize`)))
  (bind _returnvalue (`KismetMathLibrary.Dot_VectorVector` (`local.DeltaUp`) (`self.GetActorUpVector` (`GameplayStatics.GetPlayerCameraManager` 0))))
  (bind _returnvalue_2 (`KismetMathLibrary.Dot_VectorVector` (`local.DeltaRight`) (`self.GetActorRightVector` (`GameplayStatics.GetPlayerCameraManager` 0))))
  (bind (_belowmin _abovemax) (`/Game/Core/Blueprints/RSFunctionLibrary.isFloatInBounds` _y_2 (`local.Topmargin`) (- _y_3 (`local.Topmargin`))))
  (bind (_belowmin_2 _abovemax_2) (`/Game/Core/Blueprints/RSFunctionLibrary.isFloatInBounds` _x_2 (`local.Sidemargin`) (- _x_3 (`local.Sidemargin`))))
  ;[0.3968 0.3968 0.3968] To avoid flickering, the range the player can move in is slightly smaller than the entire screen
  (set `local.Sidemargin` (/ _x 10.0))
  (set `local.Topmargin` (/ _y 10.0))
  (set `local.ScreenPos` (`GameplayStatics.ProjectWorldToScreen` (`GameplayStatics.GetPlayerController` 0) (+ (+ (`local.DeltaRight`) (`local.DeltaUp`)) (`SceneComponent.K2_GetComponentLocation` (`self.Hitbox`)))))
  (return (+ (`KismetMathLibrary.SelectVector` (`KismetMathLibrary.SelectVector` (`KismetMathLibrary.SelectVector` _deltaright (0.0 0.0 0.0) (> _returnvalue_2 0.0)) (`KismetMathLibrary.SelectVector` _deltaright (0.0 0.0 0.0) (< _returnvalue_2 0.0)) _belowmin_2) (`local.DeltaRight`) (or _belowmin_2 _abovemax_2)) (`KismetMathLibrary.SelectVector` (`KismetMathLibrary.SelectVector` (`KismetMathLibrary.SelectVector` _deltaup (0.0 0.0 0.0) (< _returnvalue 0.0)) (`KismetMathLibrary.SelectVector` _deltaup (0.0 0.0 0.0) (> _returnvalue 0.0)) _belowmin) (`local.DeltaUp`) (or _belowmin _abovemax)))))

(fn `MoveIntoView`
  (params (ScreenPos :type "Vector2D Structure"))
  (returns (Delta :type "Vector Structure"))
  (bind (_x _y) (`KismetMathLibrary.BreakVector2D` ScreenPos))
  (bind _returnvalue (`GameplayStatics.GetPlayerCameraManager` 0))
  (bind _speed (`self.Speed`))
  (bind _speed_2 (`self.Speed`))
  (bind (_x_2 _y_2) (`KismetMathLibrary.BreakVector2D` (`WidgetLayoutLibrary.GetViewportSize`)))
  (bind (_belowmin _abovemax) (`/Game/Core/Blueprints/RSFunctionLibrary.isFloatInBounds` _y 0.0 _y_2))
  (bind (_belowmin_2 _abovemax_2) (`/Game/Core/Blueprints/RSFunctionLibrary.isFloatInBounds` _x 0.0 _x_2))
  ;[0.3968 0.3968 0.3968] If we're outside the viewport, move us back down/up/right/left as needed to get us back into view
  (return (+ (* (`self.GetActorRightVector` _returnvalue) (`KismetMathLibrary.SelectFloat` (`KismetMathLibrary.SelectFloat` _speed_2 (* _speed_2 -1.0) _belowmin_2) 0.0 (or _belowmin_2 _abovemax_2))) (* (`self.GetActorUpVector` _returnvalue) (`KismetMathLibrary.SelectFloat` (`KismetMathLibrary.SelectFloat` (* _speed -1.0) _speed _belowmin) 0.0 (or _belowmin _abovemax))))))

(fn `MoveShip`
  (locals (ScreenPos :type "Vector2D Structure"))
  (bind (_returnvalue _screenpos) (`/Game/Core/Blueprints/RSFunctionLibrary.IsInView` (`GameplayStatics.GetPlayerController` 0) (`SceneComponent.K2_GetComponentLocation` (`self.Hitbox`))))
  ;[0.3968 0.3968 0.3968] Is in view?
  (if _returnvalue
    ;[0.3968 0.3968 0.3968] Use Player input to move
    (`SceneComponent.K2_AddWorldOffset` (`self.Hitbox`) (`self.ClampToScreen` (* (`self.MoveRightDelta`) (`GameplayStatics.GetWorldDeltaSeconds`)) (* (`self.MoveUpDelta`) (`GameplayStatics.GetWorldDeltaSeconds`))) false false)
    (else
      ;[0.3968 0.3968 0.3968] You might want to set this False for cutscenes where you move the camera
      (if (`self.ShouldMovePlayerIntoView`)
        ;[0.3968 0.3968 0.3968] Move Player back into view
        (bind _output_get (set `local.ScreenPos` _screenpos))
        (`SceneComponent.K2_AddWorldOffset` (`self.Hitbox`) (* (`self.MoveIntoView` _output_get) (`GameplayStatics.GetWorldDeltaSeconds`)) false false)))))

(fn `SetAimPointLoc`
  (bind (_hitresult _returnvalue) (`PlayerController.GetHitResultUnderCursorByChannel` (`GameplayStatics.GetPlayerController` 0) "TraceTypeQuery3" false))
  ;[0.3968 0.3968 0.3968] Uses the ShootPoint Mesh to get a hit result, then set AimPoint to that location
  (if _returnvalue
    (`SceneComponent.K2_SetWorldLocation` (`self.AimPoint`) (`.Location` (`GameplayStatics.BreakHitResult` _hitresult)) false false)))

(fn `TraceAround`
  (bind _hitbox (`self.Hitbox`))
  (bind _returnvalue (`SceneComponent.K2_GetComponentLocation` _hitbox))
  ;[0.3968 0.3968 0.3968] Capsule Trace to see if we're flying into a static object (e.g. a Wall)
  (if (not (`self.isInvincible`))
    (bind (_outhit _returnvalue_2) (`KismetSystemLibrary.CapsuleTraceSingleForObjects` _returnvalue _returnvalue (`CapsuleComponent.GetScaledCapsuleHalfHeight` _hitbox) (`CapsuleComponent.GetScaledCapsuleRadius` _hitbox) (`|MakeArray` "ObjectTypeQuery1" :!type "EObjectTypeQuery Enum")))
    ;[0.3968 0.3968 0.3968] Deal damage if we run into stuff
    (if _returnvalue_2
      (`GameplayStatics.ApplyDamage` self 5.0))))

(fn `UserConstructionScript`
  (`parent.UserConstructionScript`))