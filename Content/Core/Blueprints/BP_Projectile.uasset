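; BP_Projectile is a projectile actor that damages what it overlaps and then destroys itself.
; Its collision overlap skips pickups, identified by tag, and its owner, then applies fixed damage attributed to the owner and destroys the projectile after a zero-length delay.
; It also destroys itself when it hits a wall or takes any damage, which lets light-gun demo shots knock it out.
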(event `self.Collision.OnComponentBeginOverlap`
  (params (OverlappedComponent :type "PrimitiveComponent Object Reference") (OtherActor :type "Actor Object Reference") (OtherComp :type "PrimitiveComponent Object Reference") (OtherBodyIndex :type Integer) (bFromSweep :type Boolean) (SweepResult :type "HitResult Structure (by ref)"))
  ;[0.3968 0.3968 0.3968] Hitting enemies (ignore pickups, deal 5 damage then destroy projectile)
  (`/Engine/EditorBlueprintResources/StandardMacros.IsValid` OtherActor
    (:`Is Valid`
      (if (and (not (`self.ActorHasTag` OtherActor "Pickup")) (!= OtherActor (`self.GetOwner`)))
        (`GameplayStatics.ApplyDamage` OtherActor 5.0 null (`self.GetOwner`))
        (`KismetSystemLibrary.Delay` 0.0)
        (`self.K2_DestroyActor`)))))

(event `self.ReceiveHit`
  (params (MyComp :type "PrimitiveComponent Object Reference") (Other :type "Actor Object Reference") (OtherComp :type "PrimitiveComponent Object Reference") (bSelfMoved :type Boolean) (HitLocation :type "Vector Structure") (HitNormal :type "Vector Structure") (NormalImpulse :type "Vector Structure") (Hit :type "HitResult Structure (by ref)"))
  ;[0.3968 0.3968 0.3968] Hitting walls
  (`self.K2_DestroyActor`))

(event `self.ReceiveAnyDamage`
  (params (Damage :type "Float (single-precision)") (DamageType :type "DamageType Object Reference") (InstigatedBy :type "Controller Object Reference") (DamageCauser :type "Actor Object Reference"))
  ;[0.3968 0.3968 0.3968] Destroy when shot (light gun demo)
  (`self.K2_DestroyActor`))

(fn `UserConstructionScript`)