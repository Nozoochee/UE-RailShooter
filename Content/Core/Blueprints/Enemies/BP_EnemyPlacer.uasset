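; BP_EnemyPlacer is a placeable spawner that creates a group of BP_SimpleEnemy actors and reports when all are dead.
; The construction script previews each transform in the Enemies array with an arrow component.
; SpawnEnemies composes those relative transforms with the actor's transform, passes the follow-player flag and tracks each spawn.
; Destroyed enemies leave the tracking array; when it empties, the placer fires OnAllEnemiesKilled and destroys itself.
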(event `SpawnEnemies`
  (for _array_element (`self.Enemies`)
    (bind _returnvalue (`|SpawnActorFromClass` "/Game/Core/Blueprints/Enemies/BP_SimpleEnemy.BP_SimpleEnemy_C" (`KismetMathLibrary.ComposeTransforms` _array_element (`self.GetTransform`)) "Undefined" "OverrideRootScale" null (`self.EnemyFollowPlayer`) null))
    ;[0.3968 0.3968 0.3968] Keep track of all the enmies we spawned and every time one of them gets destroyed, remove them from the array. When the array is empty, we know everything we spawned died and can destroy ourself
    (add `self.OnDestroyed` _returnvalue (delegate `HandleDeath`))
    (`KismetArrayLibrary.Array_Add` (`self.SpawnedEnemies`) _returnvalue)))

(event `HandleDeath` :!signature `self.OnDestroyed`
  (params (DestroyedActor :type "Actor Object Reference"))
  (bind _spawnedenemies (`self.SpawnedEnemies`))
  ;[0.3968 0.3968 0.3968] Keep track of all the enmies we spawned and every time one of them gets destroyed, remove them from the array. When the array is empty, we know everything we spawned died and can destroy ourself
  (`KismetArrayLibrary.Array_RemoveItem` _spawnedenemies DestroyedActor)
  (if (== (`KismetArrayLibrary.Array_Length` _spawnedenemies) 0)
    (`self.OnAllEnemiesKilled`)
    (`self.K2_DestroyActor`)))

(fn `UserConstructionScript`
  ;[0.3968 0.3968 0.3968] Create arrows for every transform so we know their rotation
  (for _array_element (`self.Enemies`)
    (`AddComponent|NODE_AddArrowComponent-1` :`RelativeTransform` _array_element)))