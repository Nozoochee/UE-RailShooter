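; BP_SimpleEnemy is a basic enemy that periodically fires BP_EnemyProjectile at the player's hitbox and destroys itself after a maximum lifetime.
; A looping timer, randomized once at BeginPlay, drives shooting, while a slower timer disables firing whenever the enemy is out of view.
; Damage routes into ACHealthComp, whose OnDeath destroys the actor.
; ShouldFollowPlayer optionally attaches it to the player so it moves along.
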(event `self.ReceiveBeginPlay`
  (`self.SetLifeSpan` (`self.MaxLifetime`))
  (bind _asbp_base_player (cast `/Game/Core/Blueprints/Player/BP_BasePlayer` (`GameplayStatics.GetPlayerPawn` 0)))
  (set `self.PlayerRef` _asbp_base_player)
  ;[0.3968 0.3968 0.3968] Shoot roughly every second
  (`KismetSystemLibrary.K2_SetTimer` null "ShootAtPlayer" (`KismetMathLibrary.RandomFloatInRange` 0.8 1.2) true)
  ;[0.3968 0.3968 0.3968] Don't shoot if off-screen
  (`self.Still in view`)
  (`KismetSystemLibrary.K2_SetTimerDelegate` (delegate `Still in view`) 2.0 true)
  ;[0.3968 0.3968 0.3968] Destroy when dead
  (add `/Game/Core/Blueprints/AC_HealthComp.OnDeath` (`self.AC_HealthComp`) (delegate `Die`))
  ;[1 1 1] Make enemy move with player
  (if (`self.shouldFollowPlayer`)
    (`self.K2_AttachToActor` (`self.PlayerRef`) "None" "KeepWorld" "KeepWorld" "KeepWorld")))

(event `Die`
  ;[0.3968 0.3968 0.3968] Destroy when dead
  (`self.K2_DestroyActor`))

(event `Still in view`
  ;[0.3968 0.3968 0.3968] Don't shoot if off-screen
  (set `self.isActive` (`/Game/Core/Blueprints/RSFunctionLibrary.IsInView` (`GameplayStatics.GetPlayerController` 0) (`self.K2_GetActorLocation`))))

(event `self.ReceiveAnyDamage`
  (params (Damage :type "Float (single-precision)") (DamageType :type "DamageType Object Reference") (InstigatedBy :type "Controller Object Reference") (DamageCauser :type "Actor Object Reference"))
  ;[0.3968 0.3968 0.3968] Damage
  (`/Game/Core/Blueprints/AC_HealthComp.TakeDamage` (`self.AC_HealthComp`) Damage DamageType InstigatedBy DamageCauser))

(fn `ShootAtPlayer`
  (bind _returnvalue (`SceneComponent.K2_GetComponentLocation` (`self.ShootPoint`)))
  ;[0.3968 0.3968 0.3968] Shoot towards player's hitbox
  (if (`self.isActive`)
    (`/Engine/EditorBlueprintResources/StandardMacros.IsValid` (`self.PlayerRef`)
      (:`Is Valid`
        (`|SpawnActorFromClass` "/Game/Core/Blueprints/Enemies/BP_EnemyProjectile.BP_EnemyProjectile_C" (`KismetMathLibrary.MakeTransform` _returnvalue (`KismetMathLibrary.FindLookAtRotation` _returnvalue (`SceneComponent.K2_GetComponentLocation` (`/Game/Core/Blueprints/Player/BP_BasePlayer.Hitbox` (`self.PlayerRef`))))) "AlwaysSpawn" "OverrideRootScale" self null)))))

(fn `UserConstructionScript`)