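; BP_Button is a damage-activated toggle switch with a text label showing its on or off state.
; When an actor tagged Player is the damage causer, a FlipFlop sets IsActivated and fires OnButtonChanged for listeners.
; The label is refreshed on BeginPlay and after each toggle, picking OnText or OffText into a "Going {A}" string.
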(event `self.ReceiveBeginPlay`
  (`TextRenderComponent.K2_SetText` (`self.TextRender`) (`|FormatText` "Going {A}" (`KismetMathLibrary.SelectString` (`self.OnText`) (`self.OffText`) (`self.isActivated`))) :!label _label))

(event `self.ReceiveAnyDamage`
  (params (Damage :type "Float (single-precision)") (DamageType :type "DamageType Object Reference") (InstigatedBy :type "Controller Object Reference") (DamageCauser :type "Actor Object Reference"))
  (if (`self.ActorHasTag` DamageCauser "Player")
    (bind _isa (`/Engine/EditorBlueprintResources/StandardMacros.FlipFlop`)
      (:`A`
        _)
      (:`B`
        _))
    (bind _output_get (set `self.isActivated` _isa))
    (`self.OnButtonChanged` _output_get)
    (goto _label)))

(fn `UserConstructionScript`)